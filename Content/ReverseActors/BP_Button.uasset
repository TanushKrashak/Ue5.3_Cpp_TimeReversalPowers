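; BP_Button is a button actor that the player can press once when near it.
; Its Box overlap registers and unregisters BP_Player characters with the AC_PressableAction component.
; When that component fires its Action event, a latching IsPressed flag is set and the Button component shifts slightly along local Y.
; The press triggers nothing else in this Blueprint, and nothing here resets it.
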(event OnComponentBeginOverlap(Box)
  (params (OverlappedComponent :type Primitive%20Component%20Object%20Reference) (OtherActor :type Actor%20Object%20Reference) (OtherComp :type Primitive%20Component%20Object%20Reference) (OtherBodyIndex :type Integer) (bFromSweep :type Boolean) (SweepResult :type Hit%20Result%20Structure%20%28by%20ref%29))
  (bind _asbp_player (Utilities|Casting|CastToBP_Player OtherActor))
  (Default|RegisterCharacter (Variables|Default|GetAC_PressableAction) _asbp_player))

(event OnComponentEndOverlap(Box)
  (params (OverlappedComponent :type Primitive%20Component%20Object%20Reference) (OtherActor :type Actor%20Object%20Reference) (OtherComp :type Primitive%20Component%20Object%20Reference) (OtherBodyIndex :type Integer))
  (bind _asbp_player (Utilities|Casting|CastToBP_Player OtherActor))
  (Default|UnregisterCharacter (Variables|Default|GetAC_PressableAction) _asbp_player))

(event Action(AC_PressableAction)
  (if (not (Variables|Default|GetIsPressed?))
    (Variables|Default|SetIsPressed? true)
    (Transformation|AddLocalOffset (Variables|Default|GetButton) "0.000000,4.000000,0.000000" false false)))

(event EventBeginPlay)

(event Collision|EventActorBeginOverlap
  (params (OtherActor :type Actor%20Object%20Reference)))

(event EventTick
  (params (DeltaSeconds :type Float%20%28single-precision%29)))

(fn ConstructionScript)