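; Game mode Blueprint that switches on time control through the time manager when play begins.
; BeginPlay then constructs two BP_TimePointBase objects with different values and interpolates between them at a fixed distance.
; The result is cast back to BP_TimePointBase and its value printed, which acts as a simple check of time point interpolation.
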(event EventBeginPlay
  (Class|CppTimeManager|EnableTimeControl (Class|CppTimeGameMode|GetTimeManager))
  (bind _returnvalue (Game|ConstructObjectfromClass "/Game/BP_TimePointBase.BP_TimePointBase_C"))
  (Variables|/Game/BP_TimePointBase.BP_TimePointBase_C|SetValue _returnvalue 1.0)
  (bind _returnvalue_2 (Game|ConstructObjectfromClass "/Game/BP_TimePointBase.BP_TimePointBase_C"))
  (Variables|/Game/BP_TimePointBase.BP_TimePointBase_C|SetValue _returnvalue_2 2.0)
  (bind _returnvalue_3 (Class|CppTimePointBase|Interpolate _returnvalue _returnvalue_2 0.1))
  (bind _asbp_time_point_base (Utilities|Casting|CastToBP_TimePointBase _returnvalue_3))
  (Development|PrintString (Utilities|String|ToString(Float) (Variables|/Game/BP_TimePointBase.BP_TimePointBase_C|GetValue _asbp_time_point_base)) true true "(R=0.000000,G=0.660000,B=1.000000,A=1.000000)" 2e+02))

(fn ConstructionScript)